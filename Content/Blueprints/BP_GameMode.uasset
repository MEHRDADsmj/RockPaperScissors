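; Game mode for a best-of-rounds rock-paper-scissors match between the player and an AI.
; BeginPlay adds the UI and finds the AI-tagged hand actor, whose mesh shows each random AI choice.
; RunCore scores each round with a modulo-3 comparison of player and AI choices.
; At MaxRounds it announces win, loss or tie, plays audio for win or loss, and resets the scores.
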(event Custom|AddPlayerWins
  (Math|Integer|IncrementInt (Variables|Default|GetPlayerWins)))

(event Custom|Tie
  (Development|PrintString "Tie")
  (CallFunction|ResetGame))

(event Custom|Win
  (Development|PrintString "Player won in total")
  (Audio|PlaySound2D "/Game/Assets/Audio/01-Stardust_Crusaders-_AudioTrimmer_com_.01-Stardust_Crusaders-_AudioTrimmer_com_" 1.0 1.0 0.0 0 0)
  (CallFunction|ResetGame))

(event Custom|Lose
  (Development|PrintString "AI won in total")
  (Audio|PlaySound2D "/Game/Assets/Audio/Kohta_Yamamoto_-_Ashes_on_The_Fire-_AudioTrimmer_com_.Kohta_Yamamoto_-_Ashes_on_The_Fire-_AudioTrimmer_com_" 1.0 1.0 0.0 0 0)
  (CallFunction|ResetGame))

(event Custom|AddAIWins
  (Math|Integer|IncrementInt (Variables|Default|GetAIWins)))

(event Custom|AddRoundsPlayed
  (Math|Integer|IncrementInt (Variables|Default|GetRoundsPlayed)))

(event Custom|ResetGame
  (Variables|Default|SetPlayerWins 0)
  (Variables|Default|SetAIWins 0)
  (Variables|Default|SetRoundsPlayed 0))

(event Custom|RunCore
  (bind _returnvalue (CallFunction|GetRandomWeapon))
  (bind _return (CallFunction|DetermineWinner (Variables|Default|GetPlayerChoice) _returnvalue))
  (switch int _return
    (:-1
      (CallFunction|AddAIWins))
    (:0
      _)
    (:1
      (CallFunction|AddPlayerWins)))
  (Math|Integer|IncrementInt (Variables|Default|GetRoundsPlayed)
    (:%20%20
      (if (== (Variables|Default|GetRoundsPlayed) (Variables|Default|GetMaxRounds))
        (CallFunction|CheckWinState)))))

(event EventBeginPlay
  (bind _returnvalue (UserInterface|CreateWidget "/Game/Blueprints/WBP_UI.WBP_UI_C" (Game|GetPlayerController 0)))
  (UserInterface|Viewport|AddtoViewport _returnvalue 0)
  (bind _outactors (Actor|GetAllActorswithTag "AI"))
  (bind _asbp_player_hand (Utilities|Casting|CastToBP_PlayerHand (Utilities|Array|Get(acopy) _outactors)))
  (Variables|Default|SetHand _asbp_player_hand))

(fn ConstructionScript)

(fn CheckWinState
  (if (> (Variables|Default|GetPlayerWins) (Variables|Default|GetAIWins))
    (CallFunction|Win)
    (elif (== (Variables|Default|GetPlayerWins) (Variables|Default|GetAIWins))
      (CallFunction|Tie)
      (else
        (CallFunction|Lose)))))

(fn DetermineWinner
  (params (First :type Enum_EChoice%20Enum :default "NewEnumerator0") (Second :type Enum_EChoice%20Enum :default "NewEnumerator0"))
  (if (Utilities|Enum|Equal(Enum) First Second)
    (return 0)
    (else
      (bind _returnvalue (CallFunction|IsRight First Second))
      (return (select _returnvalue -1 1)))))

(fn GetRandomWeapon
  (bind _output_get (Variables|Default|SetAIChoice (Math|Conversions|ToByte(Integer) (Math|Random|RandomIntegerinRange 0 2))))
  (Default|ChangeMesh (Variables|Default|GetHand) (Utilities|Enum|ByteToEnumEnum_EChoice _output_get))
  (Development|PrintString (Utilities|String|Append "AI:" (Utilities|String|EnumtoString (Utilities|Enum|ByteToEnumEnum_EChoice _output_get))) true true "(R=1.000000,G=0.041269,B=0.000000,A=1.000000)" 5.0)
  (return (Utilities|Enum|ByteToEnumEnum_EChoice _output_get)))

(fn IsRight
  (params (A :type Byte) (B :type Byte))
  (return (== (Class|KismetMathLibrary|PercentByteByte (+ A 1) 3) B)))