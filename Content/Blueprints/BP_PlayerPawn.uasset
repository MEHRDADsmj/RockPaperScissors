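; BP_PlayerPawn is the player's pawn for picking one of three EChoice options and handing it to the game mode.
; On BeginPlay it shows the mouse cursor and caches the first "Player"-tagged actor as its BP_PlayerHand.
; Number keys set the choice and change the hand's mesh to match.
; SubmitChoiceToGameMode, not called within this Blueprint, passes the choice to BP_GameMode, prints it and runs RunCore.
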(event EventBeginPlay
  (Variables|/Script/Engine.PlayerController|SetbShowMouseCursor (Game|GetPlayerController 0) true)
  (bind _outactors (Actor|GetAllActorswithTag "Player"))
  (bind _asbp_player_hand (Utilities|Casting|CastToBP_PlayerHand (Utilities|Array|Get(acopy) _outactors)))
  (Variables|Default|SetHand _asbp_player_hand))

(event Input|KeyboardEvents|1
  (params (Key :type Key%20Structure :default "None"))
  (:Pressed
    (bind _output_get (Variables|Default|SetChoice 0))
    (Default|ChangeMesh (Variables|Default|GetHand) (Utilities|Enum|ByteToEnumEnum_EChoice _output_get))))

(event Input|KeyboardEvents|2
  (params (Key :type Key%20Structure :default "None"))
  (:Pressed
    (bind _output_get (Variables|Default|SetChoice 1))
    (Default|ChangeMesh (Variables|Default|GetHand) (Utilities|Enum|ByteToEnumEnum_EChoice _output_get))))

(event Input|KeyboardEvents|3
  (params (Key :type Key%20Structure :default "None"))
  (:Pressed
    (bind _output_get (Variables|Default|SetChoice 2))
    (Default|ChangeMesh (Variables|Default|GetHand) (Utilities|Enum|ByteToEnumEnum_EChoice _output_get))))

(fn ConstructionScript)

(fn SubmitChoicetoGameMode
  (bind _choice (Variables|Default|GetChoice))
  (bind _returnvalue (Utilities|Enum|ByteToEnumEnum_EChoice _choice))
  (bind _asbp_game_mode (Utilities|Casting|CastToBP_GameMode (Game|GetGameMode)))
  (Variables|/Game/Blueprints/BP_GameMode.BP_GameMode_C|SetPlayerChoice _asbp_game_mode _returnvalue)
  (Development|PrintString (Utilities|String|Append "Player:" (Utilities|String|EnumtoString _returnvalue)) true true "(R=1.000000,G=0.000000,B=0.013035,A=1.000000)" 5.0)
  (Default|RunCore _asbp_game_mode))